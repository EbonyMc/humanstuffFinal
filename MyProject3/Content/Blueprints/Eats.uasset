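; Eats is a wandering AI pawn that removes Scannables it touches and awards points to the player.
; A looping timer periodically sends it via AI MoveTo to a random navigable point close to its current location.
; When its BoxForPoints overlaps a Scannables actor, it adds points to the player's MotionControllerPawn and destroys that actor.
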(event `self.ReceiveBeginPlay`
  (`KismetSystemLibrary.K2_SetTimer` null "Movement" 3.0 true))

(event `Movement`
  (`|AIMoveTo` self (`NavigationSystemV1.K2_GetRandomLocationInNavigableRadius` (`self.K2_GetActorLocation`) 100.0 null null) null 2.0))

(event `self.BoxForPoints.OnComponentBeginOverlap`
  (params (OverlappedComponent :type "PrimitiveComponent Object Reference") (OtherActor :type "Actor Object Reference") (OtherComp :type "PrimitiveComponent Object Reference") (OtherBodyIndex :type Integer) (bFromSweep :type Boolean) (SweepResult :type "HitResult Structure (by ref)"))
  (bind _asscannables (cast `/Game/Blueprints/Scannables` OtherActor))
  (bind _asmotion_controller_pawn (cast `/Game/VirtualRealityBP/Blueprints/MotionControllerPawn` (`GameplayStatics.GetPlayerPawn` 0)))
  (`/Game/VirtualRealityBP/Blueprints/MotionControllerPawn.Addingpoints` _asmotion_controller_pawn 5)
  (`self.K2_DestroyActor` _asscannables))

(fn `UserConstructionScript`)