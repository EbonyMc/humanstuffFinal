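; Double sliding door that opens when a ShoppingCarts actor enters its overlap volume and closes when one leaves.
; BeginPlay caches each panel's closed position and an open position offset in opposite directions along world Y.
; A timeline plays from start or reverses from end, moving both panels with VInterpTo, whose DeltaTime input takes the timeline track as a blend factor from the cached closed positions.
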(event `self.ReceiveTick`
  (params (DeltaSeconds :type "Float (single-precision)")))

(event `self.open or something.OnComponentBeginOverlap`
  (params (OverlappedComponent :type "PrimitiveComponent Object Reference") (OtherActor :type "Actor Object Reference") (OtherComp :type "PrimitiveComponent Object Reference") (OtherBodyIndex :type Integer) (bFromSweep :type Boolean) (SweepResult :type "HitResult Structure (by ref)"))
  (cast `/Game/Blueprints/ShoppingCarts` OtherActor)
  (bind (_direction _opendoor) (`Timeline|Timeline_0` :!via `PlayFromStart` :!label _label)
    (:`Update`
      (`SceneComponent.K2_SetWorldLocation` (`self.DoorRight`) (`KismetMathLibrary.VInterpTo` (`self.Door_right`) (`self.Door_rightopen`) _opendoor 1.0) false false)
      (`SceneComponent.K2_SetWorldLocation` (`self.DoorLeft`) (`KismetMathLibrary.VInterpTo` (`self.Door_Left`) (`self.Door_LeftOpen`) _opendoor 1.0) false false))))

(event `self.open or something.OnComponentEndOverlap`
  (params (OverlappedComponent :type "PrimitiveComponent Object Reference") (OtherActor :type "Actor Object Reference") (OtherComp :type "PrimitiveComponent Object Reference") (OtherBodyIndex :type Integer))
  (cast `/Game/Blueprints/ShoppingCarts` OtherActor)
  (goto _label :!via `ReverseFromEnd`))

(event `self.ReceiveBeginPlay`
  (bind _output_get (set `self.Door_right` (`SceneComponent.K2_GetComponentLocation` (`self.DoorRight`))))
  (set `self.Door_rightopen` (`KismetMathLibrary.MakeVector` (.x _output_get) (- (.y _output_get) 150.0) (.z _output_get)))
  (bind _output_get_2 (set `self.Door_Left` (`SceneComponent.K2_GetComponentLocation` (`self.DoorLeft`))))
  (set `self.Door_LeftOpen` (`KismetMathLibrary.MakeVector` (.x _output_get_2) (+ (.y _output_get_2) 150.0) (.z _output_get_2))))

(fn `UserConstructionScript`)