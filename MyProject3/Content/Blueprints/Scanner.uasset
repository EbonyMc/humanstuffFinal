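; Scanner Blueprint that registers items as scanned when they leave its Box trigger.
; On end overlap, a Scannables actor is flagged as scanned, its points value is stored, and a barcode beep plays at its location.
; If that same actor also casts to Spawner, its Namehere value is stored as CurrentColor.
; Begin overlap is empty, and a MotionControllerPawn cast is left unconnected.
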(event `self.Box.OnComponentBeginOverlap`
  (params (OverlappedComponent :type "PrimitiveComponent Object Reference") (OtherActor :type "Actor Object Reference") (OtherComp :type "PrimitiveComponent Object Reference") (OtherBodyIndex :type Integer) (bFromSweep :type Boolean) (SweepResult :type "HitResult Structure (by ref)"))
  ;[1 1 1] Scanning stuff
)

(event `self.Box.OnComponentEndOverlap`
  (params (OverlappedComponent :type "PrimitiveComponent Object Reference") (OtherActor :type "Actor Object Reference") (OtherComp :type "PrimitiveComponent Object Reference") (OtherBodyIndex :type Integer))
  ;[1 1 1] Scanning stuff
  (bind _asscannables (cast `/Game/Blueprints/Scannables` OtherActor))
  (set `/Game/Blueprints/Scannables.IsScanned` true _asscannables)
  (set `self.currentPointsValue` (`/Game/Blueprints/Scannables.Pointsvalue` _asscannables))
  (`GameplayStatics.PlaySoundAtLocation` "/Game/Audio/se_barcodeBeep__1_.se_barcodeBeep__1_" (`self.K2_GetActorLocation` _asscannables) (struct) 1.0 1.0 0.0 null null null)
  (bind _asspawner (cast `/Game/Blueprints/Spawner` OtherActor))
  (set `self.currentColor` (`/Game/Blueprints/Spawner.Namehere` _asspawner)))

(fn `UserConstructionScript`)