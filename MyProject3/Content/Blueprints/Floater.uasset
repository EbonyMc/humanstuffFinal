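; Floater is an actor Blueprint that makes a static mesh float vertically around its starting position.
; The construction script applies configurable Mesh and Material variables to the StaticMesh component.
; On BeginPlay it stores the mesh's world location and plays the Floating timeline, which lerps the Z position between MinFloat and MaxFloat offsets from that origin.
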(event `self.ReceiveBeginPlay`
  (bind (_object_z_origin_x _object_z_origin_y _object_z_origin_z) (`KismetMathLibrary.BreakVector` (`self.Object Z Origin`)))
  (set `self.Object Z Origin` (`SceneComponent.K2_GetComponentLocation` (`self.StaticMesh`)))
  (bind (_direction _newtrack_0) (`Timeline|floating`)
    (:`Update`
      (`SceneComponent.K2_SetWorldLocation` (`self.StaticMesh`) (`KismetMathLibrary.MakeVector` _object_z_origin_x _object_z_origin_y (`KismetMathLibrary.Lerp` (+ _object_z_origin_z (`self.Min float`)) (+ _object_z_origin_z (`self.Max Float`)) _newtrack_0)) false false))))

(fn `UserConstructionScript`
  (bind _staticmesh (`self.StaticMesh`))
  (`StaticMeshComponent.SetStaticMesh` _staticmesh (`self.Mesh`))
  (`PrimitiveComponent.SetMaterial` _staticmesh 0 (`self.Material`)))