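; An alien character that wanders while holding a pen and a clip.
; The construction script attaches the Pen and Clip components to matching sockets on its mesh.
; On BeginPlay, a looping timer calls Movement every few seconds, which sends the pawn via AI MoveTo to a random navigable point near its current location.
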(event `self.ReceiveBeginPlay`
  (`KismetSystemLibrary.K2_SetTimer` null "Movement" 3.0 true))

(event `Movement`
  (`|AIMoveTo` self (`NavigationSystemV1.K2_GetRandomLocationInNavigableRadius` (`self.K2_GetActorLocation`) 100.0 null null) null 2.0))

(fn `UserConstructionScript`
  (`SceneComponent.K2_AttachToComponent` (`self.Pen`) (`self.Mesh`) "Pen" "KeepRelative" "KeepRelative" "KeepRelative" true)
  (`SceneComponent.K2_AttachToComponent` (`self.Clip`) (`self.Mesh`) "Clip" "KeepRelative" "KeepRelative" "KeepRelative" true))