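; Scannable physics prop for motion-controller VR that can be grabbed and dropped, and awards points to the pawn when scanned, then destroys itself.
; Pickup either returns Reset items to their start location after a delay or clears float, spin and hop effects.
; Optional behavior events add conveyor-triggered floating, hopping, firework thrust or delayed explosion.
; While floating, Tick turns every level PointLight red alongside the random spin.
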(event `/Game/VirtualRealityBP/Blueprints/PickupActorInterface.Pickup`
  (params (AttachTo :type "SceneComponent Object Reference"))
  ;[1 1 1] Grab and release
  (set `self.Grabbed` true)
  (`PrimitiveComponent.SetSimulatePhysics` (`self.StaticMeshComponent`) false)
  (`SceneComponent.K2_AttachToComponent` (`self.K2_GetRootComponent`) AttachTo "None" "SnapToTarget" "SnapToTarget" "KeepWorld" true)
  (if (`self.Reset`)
    (`KismetSystemLibrary.Delay` 3.0)
    (`self.K2_SetActorLocation` (`self.Reset location`))
    (else
      (`self.Set Status Qou`))))

(event `Set GRot`
  (bind (_degrees_per_sec_min_max_x _degrees_per_sec_min_max_y) (`KismetMathLibrary.BreakVector2D` (`self.Degrees per sec min max`)))
  (bind _returnvalue (`KismetMathLibrary.RandomFloatInRange` _degrees_per_sec_min_max_x _degrees_per_sec_min_max_y))
  (bind _returnvalue_2 (`KismetMathLibrary.RandomFloatInRange` _degrees_per_sec_min_max_x _degrees_per_sec_min_max_y))
  (bind _returnvalue_3 (`KismetMathLibrary.RandomFloatInRange` _degrees_per_sec_min_max_x _degrees_per_sec_min_max_y))
  ;[1 1 1] Rotate
  (set `self.Arrow Rotate` (`KismetMathLibrary.MakeRotator` (`KismetMathLibrary.SelectFloat` _returnvalue_2 (* _returnvalue_2 -1.0) (`KismetMathLibrary.RandomBool`)) (`KismetMathLibrary.SelectFloat` _returnvalue_3 (* _returnvalue_3 -1.0) (`KismetMathLibrary.RandomBool`)) (`KismetMathLibrary.SelectFloat` _returnvalue (* _returnvalue -1.0) (`KismetMathLibrary.RandomBool`)))))

(event `/Game/VirtualRealityBP/Blueprints/PickupActorInterface.Drop`
  ;[1 1 1] Grab and release
  (`PrimitiveComponent.SetSimulatePhysics` (`self.StaticMeshComponent`) true)
  (`self.K2_DetachFromActor` "KeepWorld" "KeepRelative" "KeepWorld")
  (`KismetSystemLibrary.Delay` 0.3))

(event `self.ReceiveBeginPlay`
  (`KismetSystemLibrary.Delay` 0.2)
  (if (`self.Kill`)
    (`self.K2_DestroyActor`)
    (else
      ;[1 1 1] beginplay
      (if (`self.Reset`)
        (set `self.Reset location` (`self.K2_GetActorLocation`))
        (`PrimitiveComponent.SetSimulatePhysics` (`self.StaticMeshComponent`) true)
        (else
          (set `self.Phy` (`SceneComponent.IsSimulatingPhysics` (`self.StaticMeshComponent`) "None"))
          (`self.Grav`))))))

(event `Set Status Qou`
  ;[1 1 1] reset
  (`/Engine/EditorBlueprintResources/StandardMacros.IsValid` "Scannables"
    (:`Is Valid`
      (bind _output_get (set `self.Current` true))
      (set `self.IsFloating` false)
      (`PrimitiveComponent.SetEnableGravity` (`self.StaticMeshComponent`) _output_get)
      (set `self.Arrow Rotate` (struct))
      (set `self.HopPower` (0.0 0.0 0.0)))))

(event `Scanned`
  ;[1 1 1] Getting points and sending them
  (bind _asmotion_controller_pawn (cast `/Game/VirtualRealityBP/Blueprints/MotionControllerPawn` (`GameplayStatics.GetPlayerPawn` 0)))
  (`/Game/VirtualRealityBP/Blueprints/MotionControllerPawn.Addingpoints` _asmotion_controller_pawn (`self.Pointsvalue`))
  (`/Engine/EditorBlueprintResources/StandardMacros.IsValid` "Scannables"
    (:`Is Valid`
      (`self.K2_DestroyActor`))))

(event `Grav`
  ;[1 1 1] c
  (set `self.Tags` (`|MakeArray` (`self.ThisWillChange`)) :!label _label)
  (`KismetSystemLibrary.Delay` 0.1)
  (`/Engine/EditorBlueprintResources/StandardMacros.IsValid` "Scannables"
    (:`Is Valid`
      (goto _label))))

(event `self.Floating`
  (params (CanFloat :type Boolean)))

(event `Explode`
  (bind _returnvalue (`SceneComponent.K2_GetComponentLocation` (`self.Luigi`)))
  (`KismetSystemLibrary.Delay` 10.0)
  ;[1 1 1] Set explosionon object
  (`GameplayStatics.SpawnEmitterAtLocation` "/Game/StarterContent/Particles/P_Explosion.P_Explosion" _returnvalue)
  (bind (_outhit _returnvalue_2) (`KismetSystemLibrary.SphereTraceSingle` _returnvalue _returnvalue 100.0 "TraceTypeQuery3" true))
  (if _returnvalue_2
    (`self.K2_SetActorLocation` (`.HitActor` (`GameplayStatics.BreakHitResult` _outhit)) (0.0 0.0 -100.0) false false))
  (`self.K2_SetActorLocation` (0.0 0.0 -100.0))
  (`GameplayStatics.PlaySound2D` "/Game/Audio/Explosion_8_Bit.Explosion_8_Bit" 1.0 1.0 0.0 null null))

(event `FLoat`
  (if (not (`self.Reset`))
    (if (`self.Hitconveyor`) :!label _label_2
      (`KismetSystemLibrary.Delay` 4.0)
      ;[1 1 1] Makes object Float
      (set `self.HopPower` (0.0 0.0 0.0))
      (`PrimitiveComponent.SetEnableGravity` (`self.StaticMeshComponent`) false)
      (`self.Set GRot`)
      (set `self.IsFloating` true)
      (else
        (`KismetSystemLibrary.Delay` 0.2)
        (goto _label_2)))))

(event `self.ReceiveTick`
  (params (DeltaSeconds :type "Float (single-precision)"))
  (`self.K2_AddActorWorldRotation` (* (`self.Arrow Rotate`) 1.0))
  (if (`self.IsFloating`)
    (bind _outactors (`GameplayStatics.GetAllActorsOfClass` "/Script/Engine.PointLight"))
    (for _array_element _outactors
      (`LightComponent.SetIntensity` (`Light.LightComponent` _array_element) 0.0)
      (bind _lightcomponent (`Light.LightComponent` _array_element))
      (`LightComponent.SetLightColor` _lightcomponent (struct :`R` 1.0 :`B` 0.007388 :`A` 1.0) true)
      (`LightComponent.SetIntensity` _lightcomponent 30.0))))

(event `Hopper`
  ;[1 1 1] Hopper
  (`PrimitiveComponent.AddImpulse` (`self.StaticMeshComponent`) (`self.HopPower`) "None" true :!label _label_3)
  (`KismetSystemLibrary.Delay` 2.0)
  (goto _label_3))

(event `Firework`
  (bind (_returnvalue_x _returnvalue_y) (`KismetMathLibrary.BreakVector` (* (`SceneComponent.GetForwardVector` (`self.Arrow`)) (`SceneComponent.K2_GetComponentLocation` (`self.StaticMeshComponent`)))))
  (`KismetSystemLibrary.Delay` 5.0)
  (`PrimitiveComponent.AddImpulse` (`self.StaticMeshComponent`) (`KismetMathLibrary.MakeVector` _returnvalue_x _returnvalue_y) "None" false :!label _label_4)
  (`PrimitiveComponent.SetEnableGravity` (`self.StaticMeshComponent`) false)
  (`KismetSystemLibrary.Delay` 0.1)
  (goto _label_4))

(fn `UserConstructionScript`
  (set `self.Degrees per sec min max` (`KismetMathLibrary.MakeVector2D` 1.0 10.0)))