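; GravityControl is a Blueprint that switches the level's lighting off and on through two events, with no gravity logic in its graph.
; LightsOff zeroes every PointLight's intensity and swaps the Lights array to the LightsEmissive_Grav material; LightsOn restores intensity and LightsEmissive_Mat.
; A single PreviousIntensity variable is overwritten per light, so all lights restore to the last stored value.
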(event `Lights Off`
  (bind _outactors (`GameplayStatics.GetAllActorsOfClass` "/Script/Engine.PointLight"))
  (for _array_element _outactors
    (bind _pointlightcomponent (`PointLight.PointLightComponent` _array_element))
    (bind _output_get (set `self.previous intensity` (`LightComponentBase.Intensity` _pointlightcomponent)))
    (`LightComponent.SetIntensity` _pointlightcomponent 0.0)
    (for _array_element_2 (`self.Lights`)
      (`StaticMesh.SetMaterial` _array_element_2 0 "/Game/Materials/lightsEmissive_Grav.lightsEmissive_Grav"))))

(event `Lights On`
  (bind _outactors (`GameplayStatics.GetAllActorsOfClass` "/Script/Engine.PointLight"))
  (for _array_element _outactors
    (`LightComponent.SetIntensity` (`PointLight.PointLightComponent` _array_element) (stale `Lights Off` _output_get))
    (for _array_element_2 (`self.Lights`)
      (`StaticMesh.SetMaterial` _array_element_2 0 "/Game/Materials/lightsEmissive_Mat.lightsEmissive_Mat"))))

(fn `UserConstructionScript`)