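; AlienSpawn is a spawner that places aliens at its own location once the player has enough points.
; A looping ten-second timer calls SpawnAlien, which reads Points from the MotionControllerPawn and proceeds only past a threshold.
; A sequence then spawns an Alien and an AlienWIth under separate population caps.
; Both caps count actors of the Alien class, so the second sees any Alien just spawned.
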(event `self.ReceiveBeginPlay`
  (`KismetSystemLibrary.K2_SetTimer` null "SpawnAlien" 10.0 true))

(event `SpawnAlien`
  (bind _asmotion_controller_pawn (cast `/Game/VirtualRealityBP/Blueprints/MotionControllerPawn` (`GameplayStatics.GetPlayerPawn` 0)))
  (if (>= (`/Game/VirtualRealityBP/Blueprints/MotionControllerPawn.Points` _asmotion_controller_pawn) 250)
    (`|ExecutionSequence`
      (:`then_0`
        (bind _outactors (`GameplayStatics.GetAllActorsOfClass` "/Game/Blueprints/Alien.Alien_C"))
        (if (< (`KismetArrayLibrary.Array_Length` _outactors) 4)
          (`|SpawnActorFromClass` "/Game/Blueprints/Alien.Alien_C" (`KismetMathLibrary.Conv_VectorToTransform` (`self.K2_GetActorLocation`)) "Undefined" "OverrideRootScale" null null)))
      (:`then_1`
        (bind _outactors_2 (`GameplayStatics.GetAllActorsOfClass` "/Game/Blueprints/Alien.Alien_C"))
        (if (< (`KismetArrayLibrary.Array_Length` _outactors_2) 2)
          (`|SpawnActorFromClass` "/Game/Blueprints/AlienWIth.AlienWIth_C" (`KismetMathLibrary.Conv_VectorToTransform` (`self.K2_GetActorLocation`)) "Undefined" "OverrideRootScale" null null))))))

(fn `UserConstructionScript`)