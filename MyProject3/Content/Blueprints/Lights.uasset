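; Lights actor, apparently an unfinished mechanic for switching off the level's point lights.
; BeginPlay starts a looping one-second timer on LightOff, but that event is empty.
; Unconnected fragments check whether the MotionControllerPawn has at least ten Points, and separately zero every PointLight's intensity while spawning an unspecified actor at this actor's location per light.
; Neither fragment runs, so the lights stay unchanged.
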(event `self.ReceiveBeginPlay`
  (`KismetSystemLibrary.K2_SetTimer` null "LightOff" 1.0 true))

(event `LightOff`)

(fn `UserConstructionScript`)